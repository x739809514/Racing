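; BP_MapGenerator is an actor that cleans itself up by distance and closes its Box behind a passing car; despite the name, it spawns nothing here.
; From BeginPlay, a one-second Delay loop checks the distance to the player pawn and destroys the actor once that pawn is too far away.
; When a BP_Car stops overlapping the Box, its collision profile switches to BlockAll, so the car cannot re-enter.
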(event `self.ReceiveBeginPlay`
  (if (> (`KismetMathLibrary.VSize` (- (`self.K2_GetActorLocation` (`GameplayStatics.GetPlayerPawn` 0)) (`self.K2_GetActorLocation`))) 5000.0) :!label _label
    (`self.K2_DestroyActor`)
    (else
      (`KismetSystemLibrary.Delay` 1.0)
      (goto _label))))

(event `self.Box.OnComponentEndOverlap`
  (params (OverlappedComponent :type "PrimitiveComponent Object Reference") (OtherActor :type "Actor Object Reference") (OtherComp :type "PrimitiveComponent Object Reference") (OtherBodyIndex :type Integer))
  (cast `/Game/RACER/BluePrint/BP_Car` OtherActor)
  (`PrimitiveComponent.SetCollisionProfileName` (`self.Box`) "BlockAll" false))

(fn `UserConstructionScript`)