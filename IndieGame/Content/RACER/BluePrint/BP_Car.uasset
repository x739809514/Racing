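; BP_Car is the player car, which switches between Racer, Pilot, Soldier and Viking roles, starting as Racer.
; Overlaps on its Cube read the other actor's first tag to change role or register an Obstacle hit.
; Shoot pulls bullets from the level's BP_ObjectPool at arrow transforms: three for Pilot, one for Soldier.
; Obstacles damage a Viking through BPDamageComponent until the death UI shows, while other roles get it immediately.
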(event `self.ReceiveBeginPlay`
  (bind _outactors (`GameplayStatics.GetAllActorsOfClass` "/Game/RACER/BluePrint/BP_ObjectPool.BP_ObjectPool_C"))
  (set `self.BulletPool` (`|GetArrayItem` _outactors))
  (set `self.CurrentCharacter` "NewEnumerator1"))

(event `InputAction|shoot`
  (params (Key :type "Key Structure"))
  (:`Pressed`
    (switch `/Game/RACER/CharacterEnum` (`self.CurrentCharacter`)
      (:`NewEnumerator0`
        (`self.Generate Bullet` (`self.Arrow`))
        (`self.Generate Bullet` (`self.Arrow2`))
        (`self.Generate Bullet` (`self.Arrow3`)))
      (:`NewEnumerator3`
        (`self.Generate Bullet` (`self.Arrow`))))))

(event `self.Cube.OnComponentBeginOverlap`
  (params (OverlappedComponent :type "PrimitiveComponent Object Reference") (OtherActor :type "Actor Object Reference") (OtherComp :type "PrimitiveComponent Object Reference") (OtherBodyIndex :type Integer) (bFromSweep :type Boolean) (SweepResult :type "HitResult Structure (by ref)"))
  (bind _bp_damagecomponent (`self.BP_DamageComponent`))
  ;[1 1 1] Change Character Type
  (if (`KismetSystemLibrary.IsValid` OtherActor)
    (switch `name` (`|GetArrayItem` (`Actor.Tags` OtherActor))
      (:`Pilot`
        (set `self.CurrentCharacter` "NewEnumerator0"))
      (:`Racer`
        (set `self.CurrentCharacter` "NewEnumerator1"))
      (:`Soldier`
        (set `self.CurrentCharacter` "NewEnumerator3"))
      (:`Viking`
        (set `self.CurrentCharacter` "NewEnumerator2"))
      (:`Obstacle`
        (if (`|EnumEquality` (`self.CurrentCharacter`) "NewEnumerator2")
          (`/Game/RACER/BluePrint/BP_DamageComponent.GetDamage` _bp_damagecomponent 1.0)
          (bind _curhp (`/Game/RACER/BluePrint/BP_DamageComponent.GetCurHP` _bp_damagecomponent))
          (if (<= _curhp 0.0)
            (bind _returnvalue (`|CreateWidget` "/Game/RACER/UI/BP_DeadUI.BP_DeadUI_C"))
            (`UserWidget.AddToViewport` _returnvalue 0))
          (else
            (bind _returnvalue_2 (`|CreateWidget` "/Game/RACER/UI/BP_DeadUI.BP_DeadUI_C"))
            (`UserWidget.AddToViewport` _returnvalue_2 0)))))))

(fn `Generate Bullet`
  (params (ArrowPos :type "ArrowComponent Object Reference"))
  (`/Game/RACER/BluePrint/BP_ObjectPool.Get Objects` (`self.BulletPool`) (`SceneComponent.K2_GetComponentToWorld` ArrowPos)))

(fn `GetCurrentCharacter`
  (returns (CurCharacter :type "/Game/RACER/CharacterEnum Enum"))
  (return (`self.CurrentCharacter`)))

(fn `UserConstructionScript`)