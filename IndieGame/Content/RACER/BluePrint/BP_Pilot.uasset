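; BP_Pilot is a short-lived obstacle actor in the Racer game that destroys itself on a six-second timer started at BeginPlay.
; BeginPlay also caches whether the actor carries its configured tag.
; If tagged, Tick adds a local rotation to the Cube, built from the actor's rotation plus random, delta-scaled pitch and yaw jitter.
; A Box overlap with a Player-tagged actor hides the obstacle rather than destroying it immediately.
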(event `self.ReceiveTick`
  (params (DeltaSeconds :type "Float (single-precision)"))
  (bind (_returnvalue_roll _returnvalue_pitch _returnvalue_yaw) (`KismetMathLibrary.BreakRotator` (`self.K2_GetActorRotation`)))
  (if (`self.HasTag`)
    (`SceneComponent.K2_AddLocalRotation` (`self.Cube`) (`KismetMathLibrary.MakeRotator` _returnvalue_roll (+ _returnvalue_pitch (* (`KismetMathLibrary.RandomFloatInRange` -90.0 90.0) DeltaSeconds)) (+ _returnvalue_yaw (* (`KismetMathLibrary.RandomFloatInRange` -90.0 90.0) DeltaSeconds))) false false)))

(event `self.ReceiveBeginPlay`
  (set `self.HasTag` (`self.ActorHasTag` (`self.Tag`)))
  (`KismetSystemLibrary.K2_SetTimerDelegate` (delegate `DestroyObstacle_Event`) 6.0))

(event `DestroyObstacle_Event`
  (`self.K2_DestroyActor`))

(event `self.Box.OnComponentBeginOverlap`
  (params (OverlappedComponent :type "PrimitiveComponent Object Reference") (OtherActor :type "Actor Object Reference") (OtherComp :type "PrimitiveComponent Object Reference") (OtherBodyIndex :type Integer) (bFromSweep :type Boolean) (SweepResult :type "HitResult Structure (by ref)"))
  (if (`self.ActorHasTag` OtherActor "Player")
    (`self.SetActorHiddenInGame` true)))

(fn `UserConstructionScript`)