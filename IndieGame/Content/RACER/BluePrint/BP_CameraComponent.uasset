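; BP_CameraComponent drives a camera that follows a tagged target car along the world X axis.
; BeginPlay stores the first actor matching TargetTag as TargetCar and snaps Camera to a fixed start position.
; Each Tick moves Camera to a set offset behind the car's X, with Y and height held constant.
; A node that would set the camera's downward pitch is present but never runs.
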(event `self.ReceiveBeginPlay`
  (bind _outactors (`GameplayStatics.GetAllActorsWithTag` (`KismetStringLibrary.Conv_StringToName` (`self.TargetTag`))))
  (set `self.TargetCar` (`|GetArrayItem` _outactors))
  (`Actor.K2_SetActorLocation` (`self.camera`) (90.0 963.0 1500.0) false false))

(event `self.ReceiveTick`
  (params (DeltaSeconds :type "Float (single-precision)"))
  (`Actor.K2_SetActorLocation` (`self.camera`) (- (`KismetMathLibrary.MakeVector` (.x (`Actor.K2_GetActorLocation` (`self.TargetCar`))) 963.0 1500.0) (100.0 0.0 0.0)) false false))