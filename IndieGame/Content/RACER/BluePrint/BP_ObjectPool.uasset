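; Object pool actor that pre-spawns hidden BP_Bulllet actors on BeginPlay for reuse.
; GetObjects unhides and moves the first hidden bullet, using the hidden flag as the free marker and applying only location.
; When PoolNum hits zero it spawns another batch, then unhides the first array entry but moves the last cached Obj.
; ReturnObjects re-hides the bullet and increments the free count, leaving collision enabled.
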(event `self.ReceiveBeginPlay`
  (for _ (range (`self.PoolSize`))
    (bind _returnvalue (`|SpawnActorFromClass` "/Game/RACER/BluePrint/BP_Bulllet.BP_Bulllet_C" (`KismetMathLibrary.MakeTransform` (0.0 0.0 0.0)) "Undefined" "MultiplyWithRoot" null null))
    (if (`KismetSystemLibrary.IsValid` _returnvalue)
      (set `self.PoolNum` (+ (`self.PoolNum`) 1))
      (`self.SetActorHiddenInGame` _returnvalue true)
      (`self.SetActorEnableCollision` _returnvalue true)
      (`KismetArrayLibrary.Array_Add` (`self.PoolObejcts`) _returnvalue))))

(fn `Get Objects`
  (params (SpawnTransform :type "Transform Structure"))
  (returns (Objects :type "Actor Object Reference"))
  (bind _spawntranform_location (`KismetMathLibrary.BreakTransform` (`self.SpawnTranform`)))
  (bind _spawntranform_location_2 (`KismetMathLibrary.BreakTransform` (`self.SpawnTranform`)))
  (set `self.SpawnTranform` SpawnTransform)
  (if (> (`self.PoolNum`) 0)
    (for _array_element (`self.PoolObejcts`)
      (set `self.Obj` _array_element)
      (if (`Actor.bHidden` _array_element)
        (`self.SetActorHiddenInGame` (`self.Obj`) false)
        (`self.K2_SetActorLocation` (`self.Obj`) _spawntranform_location_2 false false)
        (set `self.PoolNum` (- (`self.PoolNum`) 1))
        (return null)))
    (else
      (for _ (range 11)
        (bind _returnvalue (`|SpawnActorFromClass` "/Game/RACER/BluePrint/BP_Bulllet.BP_Bulllet_C" (`self.SpawnTranform`) "Undefined" "MultiplyWithRoot" null null))
        (if (`KismetSystemLibrary.IsValid` _returnvalue)
          (set `self.PoolNum` (+ (`self.PoolNum`) 1))
          (`self.SetActorHiddenInGame` _returnvalue true)
          (`self.SetActorEnableCollision` _returnvalue true)
          (`KismetArrayLibrary.Array_Add` (`self.PoolObejcts`) _returnvalue)))
      (`self.SetActorHiddenInGame` (`|GetArrayItem` (`self.PoolObejcts`)) false)
      (`self.K2_SetActorLocation` (`self.Obj`) _spawntranform_location false false)
      (set `self.PoolNum` (- (`self.PoolNum`) 1))
      (return null))))

(fn `ReturnObjects`
  (params (Object :type "/Game/RACER/BluePrint/BP_Bulllet Object Reference"))
  (if (`KismetSystemLibrary.IsValid` Object)
    (`self.SetActorHiddenInGame` Object true)
    (`self.SetActorEnableCollision` Object true)
    (set `self.PoolNum` (+ (`self.PoolNum`) 1))))

(fn `UserConstructionScript`)