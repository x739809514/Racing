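; BP_Bulllet is a pooled bullet actor that returns itself to BP_ObjectPool for reuse.
; On BeginPlay it finds and caches the first BP_ObjectPool in the level.
; When its sphere begins overlapping a valid actor tagged Obstacle, it returns to the pool immediately.
; An overlap with any other valid actor starts a short timer that returns it afterwards, so recycling here is triggered only by overlaps.
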(event `self.ReceiveBeginPlay`
  (bind _outactors (`GameplayStatics.GetAllActorsOfClass` "/Game/RACER/BluePrint/BP_ObjectPool.BP_ObjectPool_C"))
  (bind _output (`|GetArrayItem` _outactors))
  (if (`KismetSystemLibrary.IsValid` _output)
    (set `self.BulletPool` _output)))

(event `self.Sphere1.OnComponentBeginOverlap`
  (params (OverlappedComponent :type "PrimitiveComponent Object Reference") (OtherActor :type "Actor Object Reference") (OtherComp :type "PrimitiveComponent Object Reference") (OtherBodyIndex :type Integer) (bFromSweep :type Boolean) (SweepResult :type "HitResult Structure (by ref)"))
  (if (`KismetSystemLibrary.IsValid` OtherActor)
    (if (`self.ActorHasTag` OtherActor "Obstacle")
      (`/Game/RACER/BluePrint/BP_ObjectPool.ReturnObjects` (`self.BulletPool`) self)
      (else
        (`KismetSystemLibrary.K2_SetTimerDelegate` (delegate `RecyleBullet_Event`) 3.0)))))

(event `RecyleBullet_Event`
  (`/Game/RACER/BluePrint/BP_ObjectPool.ReturnObjects` (`self.BulletPool`) self))

(fn `UserConstructionScript`)