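; BP_CarMoverComponent is a component that drives its owning car forward and steers it sideways in a racer.
; Tick offsets the car along local X by a step that grows with time since BeginPlay, without delta-time scaling.
; Left and right inputs unpause or pause looping timers, created paused at BeginPlay, that nudge it along local Y.
; All movement uses direct local offsets without sweep, so it ignores blocking collision.
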(event `MoveRight_Event`
  (`Actor.K2_AddActorLocalOffset` (`self.GetOwner`) (0.0 5.0 0.0) false false))

(event `MoveLeft_Event`
  (`Actor.K2_AddActorLocalOffset` (`self.GetOwner`) (0.0 -5.0 0.0) false false))

(event `self.ReceiveBeginPlay`
  (set `self.StartTime` (`KismetSystemLibrary.GetGameTimeInSeconds`))
  (set `self.TargetCar` (`self.GetOwner`))
  (bind _returnvalue (`KismetSystemLibrary.K2_SetTimerDelegate` (delegate `MoveRight_Event`) 0.01 true))
  (`KismetSystemLibrary.K2_PauseTimerHandle` _returnvalue)
  (bind _returnvalue_2 (`KismetSystemLibrary.K2_SetTimerDelegate` (delegate `MoveLeft_Event`) 0.01 true))
  (`KismetSystemLibrary.K2_PauseTimerHandle` _returnvalue_2))

(event `InputAction|right`
  (params (Key :type "Key Structure"))
  (:`Pressed`
    (`KismetSystemLibrary.K2_UnPauseTimerHandle` (stale `self.ReceiveBeginPlay` _returnvalue)))
  (:`Released`
    (`KismetSystemLibrary.K2_PauseTimerHandle` (stale `self.ReceiveBeginPlay` _returnvalue))))

(event `InputAction|left`
  (params (Key :type "Key Structure"))
  (:`Pressed`
    (`KismetSystemLibrary.K2_UnPauseTimerHandle` (stale `self.ReceiveBeginPlay` _returnvalue_2)))
  (:`Released`
    (`KismetSystemLibrary.K2_PauseTimerHandle` (stale `self.ReceiveBeginPlay` _returnvalue_2))))

(event `self.ReceiveTick`
  (params (DeltaSeconds :type "Float (single-precision)"))
  (`Actor.K2_AddActorLocalOffset` (`self.TargetCar`) (`KismetMathLibrary.MakeVector` (+ (* (- (`KismetSystemLibrary.GetGameTimeInSeconds`) (`self.StartTime`)) 0.1) 10.0)) false false))