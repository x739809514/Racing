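; BP_DamageComponent is a health component that tracks the current hit points of its owner.
; On BeginPlay it initializes current HP from the configured HP value.
; GetDamage subtracts incoming damage and prints a debug message, ignoring hits once HP is at or below zero.
; GetCurHP exposes the current value; HP is not clamped and no death event fires.
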(event `self.ReceiveBeginPlay`
  (set `self.CurHP` (`self.HP`)))

(fn `GetCurHP`
  (returns (CurHP :type "Float (double-precision)"))
  (return (`self.CurHP`)))

(fn `GetDamage`
  (params (Damage :type "Float (double-precision)"))
  (if (<= (`self.CurHP`) 0.0)
    (return)
    (else
      (set `self.CurHP` (- (`self.CurHP`) Damage))
      (`KismetSystemLibrary.PrintString` "Damage!!")
      (return))))