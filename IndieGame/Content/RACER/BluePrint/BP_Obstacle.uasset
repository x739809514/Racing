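; BP_Obstacle is a destructible obstacle for the racing game that removes itself on a ten-second timer.
; Unless it carries a configurable actor tag, its cube tumbles every tick with random pitch and yaw added to the actor's rotation.
; Box overlaps with Bullet-tagged actors damage it through BPDamageComponent until HP runs out.
; A player BP_Car destroys it on overlap when its current character matches one enum value, commented as Viking.
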(event `self.ReceiveTick`
  (params (DeltaSeconds :type "Float (single-precision)"))
  (bind (_returnvalue_roll _returnvalue_pitch _returnvalue_yaw) (`KismetMathLibrary.BreakRotator` (`self.K2_GetActorRotation`)))
  (if (not (`self.HasTag`))
    (`SceneComponent.K2_AddLocalRotation` (`self.Cube`) (`KismetMathLibrary.MakeRotator` _returnvalue_roll (+ _returnvalue_pitch (* (`KismetMathLibrary.RandomFloatInRange` -90.0 90.0) DeltaSeconds)) (+ _returnvalue_yaw (* (`KismetMathLibrary.RandomFloatInRange` -90.0 90.0) DeltaSeconds))) false false)))

(event `DestroyObstacle_Event`
  ;[1 1 1] Destroy Obstacle, Todo: Change to destroy after obstacle out of view
  (`self.K2_DestroyActor`))

(event `self.ReceiveBeginPlay`
  (set `self.HasTag` (`self.ActorHasTag` (`self.Tag`)))
  ;[1 1 1] Destroy Obstacle, Todo: Change to destroy after obstacle out of view
  (`KismetSystemLibrary.K2_SetTimerDelegate` (delegate `DestroyObstacle_Event`) 10.0 true))

(event `self.Box.OnComponentBeginOverlap`
  (params (OverlappedComponent :type "PrimitiveComponent Object Reference") (OtherActor :type "Actor Object Reference") (OtherComp :type "PrimitiveComponent Object Reference") (OtherBodyIndex :type Integer) (bFromSweep :type Boolean) (SweepResult :type "HitResult Structure (by ref)"))
  (bind _bp_damagecomponent (`self.BP_DamageComponent`))
  (if (`KismetSystemLibrary.IsValid` OtherActor)
    (bind _output_get (set `self.TargetActor` OtherActor))
    (if (`self.ActorHasTag` _output_get "Bullet")
      (`/Game/RACER/BluePrint/BP_DamageComponent.GetDamage` _bp_damagecomponent 1.0)
      (bind _curhp (`/Game/RACER/BluePrint/BP_DamageComponent.GetCurHP` _bp_damagecomponent))
      (if (<= _curhp 0.0)
        (`self.K2_DestroyActor`))
      (else
        ;[1 1 1] Viking Vs Obstacle
        (if (`self.ActorHasTag` (`self.TargetActor`) "Player")
          (bind _asbp_car (cast `/Game/RACER/BluePrint/BP_Car` (`self.TargetActor`)))
          (bind _curcharacter (`/Game/RACER/BluePrint/BP_Car.GetCurrentCharacter` _asbp_car))
          (if (`|EnumEquality` _curcharacter "NewEnumerator2")
            (`self.K2_DestroyActor`)))))))

(fn `UserConstructionScript`)